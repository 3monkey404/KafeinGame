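; PC_Dreamer is a player controller that sets game-only input and manages the pause menu and interaction prompt widgets.
; On BeginPlay it adds the default Enhanced Input mapping context, then creates both widgets and adds them to the viewport hidden.
; The pause input hides the interaction prompt and calls the pause menu's Pause, while ShowInteraction and HideInteraction events toggle the prompt's visibility.
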(event `self.ReceiveBeginPlay`
  (bind _returnvalue (subsystem `EnhancedInputLocalPlayerSubsystem`))
  (`WidgetBlueprintLibrary.SetInputMode_GameOnly` self)
  (`/Engine/EditorBlueprintResources/StandardMacros.IsValid` _returnvalue
    (:`Is Valid`
      (`EnhancedInputSubsystemInterface.AddMappingContext` _returnvalue "/Game/Blueprint/Input/IMC_Default.IMC_Default" 0 (struct))
      (`|ExecutionSequence`
        (:`then_0`
          (bind _returnvalue_2 (`|CreateWidget` "/Game/Widgets/W_Pause.W_Pause_C" self))
          (bind _output_get (set `self._pauseMenu` _returnvalue_2))
          (`UserWidget.AddToViewport` _output_get 0)
          (`Widget.SetVisibility` _output_get "Hidden"))
        (:`then_1`
          (bind _returnvalue_3 (`|CreateWidget` "/Game/Widgets/W_Interact.W_Interact_C" self))
          (bind _output_get_2 (set `self._interactWidget` _returnvalue_3))
          (`UserWidget.AddToViewport` _output_get_2 0)
          (`Widget.SetVisibility` _output_get_2 "Hidden"))))))

(event `EnhancedInput|/Game/Blueprint/Input/Actions/IA_Pause`
  (params (ActionValue :type Boolean) (ElapsedSeconds :type "Float (double-precision)") (TriggeredSeconds :type "Float (double-precision)") (InputAction :type "InputAction Object Reference" :default "/Game/Blueprint/Input/Actions/IA_Pause.IA_Pause"))
  (:`Triggered`
    (`self.HideInteraction`)
    (`/Game/Widgets/W_Pause.Pause` (`self._pauseMenu`))))

(event `ShowInteraction`
  (`Widget.SetVisibility` (`self._interactWidget`) "Visible"))

(event `HideInteraction`
  (`Widget.SetVisibility` (`self._interactWidget`) "Hidden"))

(fn `UserConstructionScript`)
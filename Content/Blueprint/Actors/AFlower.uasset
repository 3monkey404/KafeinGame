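; AFlower is an interactable flower actor that, when picked, sends the player back to the level's PlayerStart.
; StartInteraction calls CallPicked, teleports the player pawn to the location and rotation of the first PlayerStart found, then destroys the flower after a short delay.
; The construction script assembles the look from stem, center and petal mesh variables, adding an optional second petal component that shares the petal material.
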(event `/Game/Blueprint/Core/I_Interactive.StartInteraction`
  (params (Instigator :type "/Game/Blueprint/C_Dreamer Object Reference"))
  (`self.Picked`)
  (bind _returnvalue (`GameplayStatics.GetActorOfClass` "/Script/Engine.PlayerStart"))
  (`self.K2_SetActorLocationAndRotation` (`GameplayStatics.GetPlayerPawn` 0) (`self.K2_GetActorLocation` _returnvalue) (`self.K2_GetActorRotation` _returnvalue) false true)
  (`KismetSystemLibrary.Delay` 0.2)
  (`self.K2_DestroyActor`))

(fn `UserConstructionScript`
  (bind _petales1 (`self.petales1`))
  (`|ExecutionSequence`
    (:`then_0`
      (`StaticMeshComponent.SetStaticMesh` (`self.tige`) (`self.TigeVisual`)))
    (:`then_1`
      (`StaticMeshComponent.SetStaticMesh` (`self.point`) (`self.PointVisual`)))
    (:`then_2`
      (`StaticMeshComponent.SetStaticMesh` _petales1 (`self.Petal1Visual`))
      (`PrimitiveComponent.SetMaterial` _petales1 0 (`self.PetalMat`)))
    (:`then_3`
      (if (`self.Has2ndPetal`)
        (bind _returnvalue (`AddComponent|NODE_AddStaticMeshComponent-0` :`RelativeTransform` (`KismetMathLibrary.MakeTransform` (0.0 0.0 0.0))))
        (`StaticMeshComponent.SetStaticMesh` _returnvalue (`self.Petal2Visual`))
        (`PrimitiveComponent.SetMaterial` _returnvalue 0 (`self.PetalMat`))))))
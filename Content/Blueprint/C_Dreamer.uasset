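; C_Dreamer is a player-controlled character Blueprint with basic Enhanced Input movement, look and jump.
; BeginPlay adds IMC_Default to player 0's input subsystem.
; Move input is relative to the camera, deriving forward from the camera's right vector crossed with world up so pitch does not affect it.
; Look feeds controller yaw and inverted pitch, while the jump action's value selects Jump or StopJumping.
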(event `self.ReceiveBeginPlay`
  (bind _returnvalue (pcsubsystem `EnhancedInputLocalPlayerSubsystem` (`GameplayStatics.GetPlayerController` 0)))
  (`/Engine/EditorBlueprintResources/StandardMacros.IsValid` _returnvalue
    (:`Is Valid`
      (`EnhancedInputSubsystemInterface.AddMappingContext` _returnvalue "/Game/Blueprint/Input/IMC_Default.IMC_Default" 0 (struct)))))

(event `EnhancedInput|/Game/Blueprint/Input/Actions/IA_Move`
  (params (ActionValue :type "Vector2D Structure") (ElapsedSeconds :type "Float (double-precision)") (TriggeredSeconds :type "Float (double-precision)") (InputAction :type "InputAction Object Reference" :default "/Game/Blueprint/Input/Actions/IA_Move.IA_Move"))
  (bind _returnvalue (`SceneComponent.GetRightVector` (`self.Camera`)))
  (:`Triggered`
    (`self.AddMovementInput` (+ (* ActionValue_X _returnvalue) (* ActionValue_Y (`KismetMathLibrary.Cross_VectorVector` _returnvalue (`KismetMathLibrary.Vector_Up`)))))))

(event `EnhancedInput|/Game/Blueprint/Input/Actions/IA_Look`
  (params (ActionValue :type "Vector2D Structure") (ElapsedSeconds :type "Float (double-precision)") (TriggeredSeconds :type "Float (double-precision)") (InputAction :type "InputAction Object Reference" :default "/Game/Blueprint/Input/Actions/IA_Look.IA_Look"))
  (:`Triggered`
    (`self.AddControllerYawInput` ActionValue_X)
    (`self.AddControllerPitchInput` (* ActionValue_Y -1.0))))

(event `EnhancedInput|/Game/Blueprint/Input/Actions/IA_Jump`
  (params (ActionValue :type Boolean) (ElapsedSeconds :type "Float (double-precision)") (TriggeredSeconds :type "Float (double-precision)") (InputAction :type "InputAction Object Reference" :default "/Game/Blueprint/Input/Actions/IA_Jump.IA_Jump"))
  (:`Triggered`
    (if ActionValue
      (`self.Jump`)
      (else
        (`self.StopJumping`)))))

(fn `UserConstructionScript`)
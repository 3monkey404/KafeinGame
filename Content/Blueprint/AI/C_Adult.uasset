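; C_Adult is an AI-controlled adult character that avoids splashes.
; A Splashed event or a capsule overlap with an A_Splash actor passes the source to Avoid on its AI_Controller.
; SetSpeed sets max walk speed, treating a negative value as a request for DefaultSpeed, which the construction script uses to apply the default.
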(event `Splashed`
  (params (By :type "/Game/Blueprint/Actors/A_Splash Object Reference"))
  (bind _asai_controller (cast `/Game/Blueprint/AI/AI_Controller` (`AIBlueprintHelperLibrary.GetAIController` self)))
  (`/Game/Blueprint/AI/AI_Controller.Avoid` _asai_controller By))

(event `self.CapsuleComponent.OnComponentBeginOverlap`
  (params (OverlappedComponent :type "PrimitiveComponent Object Reference") (OtherActor :type "Actor Object Reference") (OtherComp :type "PrimitiveComponent Object Reference") (OtherBodyIndex :type Integer) (bFromSweep :type Boolean) (SweepResult :type "HitResult Structure (by ref)"))
  (bind _asa_splash (cast `/Game/Blueprint/Actors/A_Splash` OtherActor))
  (bind _asai_controller (cast `/Game/Blueprint/AI/AI_Controller` (`AIBlueprintHelperLibrary.GetAIController` self)))
  (`/Game/Blueprint/AI/AI_Controller.Avoid` _asai_controller _asa_splash))

(fn `SetSpeed`
  (params (NewSpeed :type "Float (double-precision)"))
  (set `CharacterMovementComponent.MaxWalkSpeed` (`KismetMathLibrary.SelectFloat` NewSpeed (`self.DefaultSpeed`) (>= NewSpeed 0.0)) (`self.CharacterMovement`)))

(fn `UserConstructionScript`
  (`self.SetSpeed` -1.0))